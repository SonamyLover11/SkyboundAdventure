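; Interactable door that, when unlocked, plays a timeline on interact, then automatically reverses it after a short delay.
; The timeline lerps the pivot's relative Z location, its sign chosen by a dot product of player direction and door forward.
; A box trigger sends a drop message to the player and teleports overlapping physics pickups to MovePickup.
; The construction script tints the door with PickupColor through a dynamic material.
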(event `self.Box.OnComponentBeginOverlap`
  (params (OverlappedComponent :type "PrimitiveComponent Object Reference") (OtherActor :type "Actor Object Reference") (OtherComp :type "PrimitiveComponent Object Reference") (OtherBodyIndex :type Integer) (bFromSweep :type Boolean) (SweepResult :type "HitResult Structure (by ref)"))
  (bind _asbp_physics_pickup (cast `/Game/Interactables/BP_PhysicsPickup` OtherActor))
  (message `/Game/Interfaces/Interface_Interact.INT_Drop` (`self.As Player Char`))
  (`self.K2_SetActorLocation` _asbp_physics_pickup (`SceneComponent.K2_GetComponentLocation` (`self.MovePickup`)) false false))

(event `/Game/Interfaces/Interface_Interact.INT_Interact`
  (params (PlayerRef :type "/Game/Player/BP_PlayerChar Object Reference"))
  (if (`self.isUnlocked?`)
    (bind _returnvalue (`self.UpdateDoorAngle` PlayerRef))
    (bind (_direction _alpha) (`Timeline|Door Plot` :!via `PlayFromStart` :!label _label)
      (:`Update`
        (`SceneComponent.K2_SetRelativeLocation` (`self.Pivot`) (`KismetMathLibrary.MakeVector` 0.0 0.0 (`KismetMathLibrary.Lerp` 0.0 _returnvalue _alpha)) false false))
      (:`Finished`
        (if (`|EnumEquality` _direction "Forward")
          (`KismetSystemLibrary.Delay` 1.0)
          (`self.ReverseTimeline`))))))

(event `ReverseTimeline`
  (goto _label :!via `ReverseFromEnd`))

(fn `UpdateDoorAngle`
  (params (self2 :type "Actor Object Reference"))
  (returns (ReturnValue :type "Float (double-precision)"))
  (return (select `bool` (> (`KismetMathLibrary.Dot_VectorVector` (`KismetMathLibrary.GetDirectionUnitVector` (`self.K2_GetActorLocation` self2) (`self.K2_GetActorLocation`)) (`self.GetActorForwardVector`)) 0.0) :`false` -90.0 :`true` 90.0)))

(fn `UserConstructionScript`
  (bind _returnvalue (`PrimitiveComponent.CreateDynamicMaterialInstance` (`self.Door`) 0 "/Game/Interactables/AnimatedInteractables/MAT_Color.MAT_Color" "None"))
  (bind _output_get (set `self.ColorDMI` _returnvalue))
  (`MaterialInstanceDynamic.SetVectorParameterValue` _output_get "Color" (`self.PickupColor`)))